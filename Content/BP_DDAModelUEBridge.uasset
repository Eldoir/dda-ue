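; Blueprint bridge to the SWDDAModel dynamic difficulty adjustment model, exposing player, challenge and algorithm settings to the game.
; BeginPlay builds the model with a local CSV data manager, player and challenge IDs, then seeds the PM algorithm with a starting theta.
; Attempts are forwarded to the model, which computes new difficulty parameters for a target difficulty after re-applying the selected algorithm.
; ID setters only change local variables, and SetPlayerGender always stores an empty string.
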(event `self.ReceiveBeginPlay`
  (bind _returnvalue (`|GenericCreateObject` "/Script/Swarms.SWDDAModel" self))
  (bind _output_get (set `self.DDAModel` _returnvalue))
  (bind _returnvalue_2 (`|GenericCreateObject` "/Script/Swarms.SWDDADataManager_LocalCSV" self))
  (`SWDDAModel.Init` _output_get _returnvalue_2 (`self.PlayerId`) (`self.ChallengeId`))
  (`SWDDAModel.setDdaAlgorithm` _output_get (`self.Algorithm`))
  (`self.InitPMAlgorithm` (`self.ThetaStart`)))

(fn `AddLastAttempt`
  (params (Attempt :type "SWDDAAttempt Object Reference"))
  (`SWDDAModel.addLastAttempt` (`self.DDAModel`) Attempt))

(fn `CheckDataAgainst`
  (params (Attempts :type "Array of SWDDAAttempt Object Reference"))
  (returns (IsSame :type Boolean))
  ;[1 1 1] For test purpose only
  (return (`SWDDAModel.checkDataAgainst` (`self.DDAModel`) Attempts)))

(fn `ComputeNewDiffParams`
  (params (TargetDifficulty :type "Float (double-precision)") (DoNotUpdateLRAccuracy :type Boolean))
  (returns (DiffParams :type "SWDiffParams Structure"))
  (bind _ddamodel (`self.DDAModel`))
  (`SWDDAModel.setDdaAlgorithm` _ddamodel (`self.Algorithm`))
  (bind _returnvalue (`SWDDAModel.computeNewDiffParams` _ddamodel TargetDifficulty (or DoNotUpdateLRAccuracy (`self.DoNotUpdateAccuracy`))))
  (return _returnvalue))

(fn `GetChallengeId`
  (returns (ChallengeId :type String))
  (return (`self.ChallengeId`)))

(fn `GetDDAAlgorithm`
  (returns (Algorithm :type "ESWDDAAlgorithm Enum"))
  (return (`self.Algorithm`)))

(fn `GetPlayerAge`
  (returns (PlayerAge :type String))
  (return (`self.PlayerAge`)))

(fn `GetPlayerGender`
  (returns (PlayerGender :type String))
  (return (`self.PlayerGender`)))

(fn `GetPlayerId`
  (returns (PlayerId :type String))
  (return (`self.PlayerId`)))

(fn `InitPMAlgorithm`
  (params (LastTheta :type "Float (double-precision)") (WonLastTime :type Boolean))
  (`SWDDAModel.setPMInit` (`self.DDAModel`) LastTheta WonLastTime))

(fn `SetChallengeId`
  (params (ChallengeId :type String))
  (set `self.ChallengeId` ChallengeId))

(fn `SetDDAAlgorithm`
  (params (Algorithm :type "ESWDDAAlgorithm Enum" :default "DDA_LOGREG"))
  (set `self.Algorithm` Algorithm))

(fn `SetPlayerAge`
  (params (PlayerAge :type String))
  (set `self.PlayerAge` PlayerAge))

(fn `SetPlayerGender`
  (params (PlayerGender :type String))
  (set `self.PlayerGender` ""))

(fn `SetPlayerId`
  (params (PlayerId :type String))
  (set `self.PlayerId` PlayerId))

(fn `UserConstructionScript`)