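; BP_DataTester is a test actor for saving and loading data in a DDA model, reporting pass or fail on screen.
; TestDataSaveAndLoad builds random challenge and player IDs from a glyph string and assigns them to the DDA object.
; It then feeds in hundreds of random SWDDAAttempt objects, keeps a parallel copy, and calls CheckDataAgainst to compare the saved data with that copy.
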(fn `TestDataSaveAndLoad`
  (locals (ChallengeId :type String :default "Ch_") (PlayerId :type String :default "Pl_") (Diff :type "Float (double-precision)"))
  (bind _returnvalue (`KismetStringLibrary.GetCharacterArrayFromString` (`self.Glyphs`)))
  (bind _output (`|GetArrayItem` _returnvalue (`KismetMathLibrary.RandomInteger` (`KismetArrayLibrary.Array_Length` _returnvalue))))
  (`|ExecutionSequence`
    (:`then_0`
      (for _ (range 20)
        (set `local.ChallengeId` (`KismetStringLibrary.Concat_StrStr` (`local.ChallengeId`) _output))))
    (:`then_1`
      (for _ (range 20)
        (set `local.PlayerId` (`KismetStringLibrary.Concat_StrStr` (`local.PlayerId`) _output))))
    (:`then_2`
      (`/Game/SWARMS/DDA/BP_DDAModelUEBridge.SetChallengeId` (`self.Dda`) (`local.ChallengeId`))
      (`/Game/SWARMS/DDA/BP_DDAModelUEBridge.SetPlayerId` (`self.Dda`) (`local.PlayerId`))
      (`KismetArrayLibrary.Array_Clear` (`self.Attempts`))
      (`KismetSystemLibrary.PrintString` "Adding data to model, to make it save them")
      (for _ (range 500)
        (bind _returnvalue_2 (`|GenericCreateObject` "/Script/Swarms.SWDDAAttempt" self))
        (bind _output_get (set `local.Diff` (`KismetMathLibrary.RandomFloat`)))
        (set `SWDDAAttempt.Result` (`KismetMathLibrary.SelectFloat` 1.0 0.0 (> _output_get 0.5)) _returnvalue_2)
        (set `SWDDAAttempt.Thetas` (`|MakeArray` _output_get) _returnvalue_2)
        (`/Game/SWARMS/DDA/BP_DDAModelUEBridge.AddLastAttempt` (`self.Dda`) _returnvalue_2)
        (`KismetArrayLibrary.Array_Add` (`self.Attempts`) _returnvalue_2))
      (`KismetSystemLibrary.PrintString` "Comparing saved data to actual ones")
      (bind _issame (`/Game/SWARMS/DDA/BP_DDAModelUEBridge.CheckDataAgainst` (`self.Dda`) (`self.Attempts`)))
      (`KismetSystemLibrary.PrintString` (`KismetMathLibrary.SelectString` "Test ok" "Test Data FAILED !" _issame)))))

(fn `UserConstructionScript`)