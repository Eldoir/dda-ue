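; Test simulator that exercises the dynamic difficulty adjustment (DDA) model with a virtual player, optionally showing its debug widget.
; Each try requests a theta from Dda, compares it to PlayerLevel plus noise, logs metrics and feeds the result back as an attempt.
; Junk variants override outcomes with random, always-win or always-fail data.
; The Gaussian helper uses polar-style rejection sampling but zeroes S before returning, so its noise is zero.
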(event `self.ReceiveBeginPlay`
  (if (`self.ShowWidgetOnBeginPlay`)
    (bind _returnvalue (`|CreateWidget` "/Game/SWARMS/DDA/WBP_DDA.WBP_DDA_C"))
    (`UserWidget.AddToViewport` _returnvalue 0)))

(fn `GetRandomNormalGaussian`
  (returns (ReturnValue :type "Float (double-precision)"))
  (locals (v1 :type "Float (double-precision)") (v2 :type "Float (double-precision)") (s :type "Float (double-precision)"))
  (bind _s (`local.s`))
  (bind _returnvalue (- (* (`KismetMathLibrary.RandomFloat`) 2.0) 1.0))
  (`self.DoWhileLoop` (or (>= _s 1.0) (== _s 0.0))
    (:`LoopBody`
      (`|ExecutionSequence`
        (:`then_0`
          (set `local.v1` _returnvalue))
        (:`then_1`
          (set `local.v2` _returnvalue))
        (:`then_2`
          (set `local.s` (+ (`KismetMathLibrary.Square` (`local.v1`)) (`KismetMathLibrary.Square` (`local.v2`)))))))
    (:`Completed`
      (bind _output_get (set `local.s` 0.0))
      (return (* _output_get (`local.v1`))))))

(fn `PlayerPlays`
  (params (ThetaDiff :type "Float (double-precision)"))
  (returns (ReturnValue :type Boolean))
  (locals (TryResult :type "Float (double-precision)"))
  ;[1 1 1] Le joueur joue au challenge.
  ; Pour un vrai jeu on utilise la variable en entrée pour faire un LERP sur les params du jeu
  (bind _output_get (set `local.TryResult` (+ (* (`self.GetRandomNormalGaussian`) 0.2) (`self.PlayerLevel`))))
  (return (> _output_get ThetaDiff)))

(fn `SimulatePlayerTries`
  (params (NbTries :type Integer))
  (`self.SimulatePlayerTriesWithJunkDataType` NbTries))

(fn `SimulatePlayerTriesJunk`
  (params (NbTries :type Integer))
  (`self.SimulatePlayerTriesWithJunkDataType` NbTries 1))

(fn `SimulatePlayerTriesJunkFail`
  (params (NbTries :type Integer))
  (`self.SimulatePlayerTriesWithJunkDataType` NbTries 3))

(fn `SimulatePlayerTriesJunkWin`
  (params (NbbTries :type Integer))
  (`self.SimulatePlayerTriesWithJunkDataType` NbbTries 2))

(fn `SimulatePlayerTriesWithJunkDataType`
  (params (NbTries :type Integer) (JunkDataType :type Integer))
  (locals (NextDiff :type "Float (double-precision)" :default 0.2) (DiffParams :type "SWDiffParams Structure") (Win :type Boolean) (Attempt :type "SWDDAAttempt Object Reference"))
  (for _ (range NbTries)
    ;[1 1 1] On demande au modèle de nous donner le bon paramètre theta en fonction de la proba voulue
    (bind _diffparams (`/Game/SWARMS/DDA/BP_DDAModelUEBridge.ComputeNewDiffParams` (`self.Dda`) (`local.NextDiff`) false))
    (bind _output_get (set `local.DiffParams` _diffparams))
    (`KismetSystemLibrary.PrintString` (`KismetTextLibrary.Conv_TextToString` (`|FormatText` "New game ! \nDifficulty: {TargetDiff} \nDifficulty with explo: {TargetDiffWithExplo} \nTheta : {Theta} \nAlgorithm Wanted: {AlgorithmWanted} \nAlgorithm Used: {AlgorithmActuallyUsed} \nLog Reg Ready: {LogRegReady} \nLog Reg Accuracy: {LRAccuracy} \nNb Attemps Used: {NbAttemptsUsedToCompute}" (break `SWDiffParams` _output_get) (`.TargetDiffWithExplo` (break `SWDiffParams` _output_get)) (`.Theta` (break `SWDiffParams` _output_get)) (`|GetEnumeratorNameAsString` (`.AlgorithmActuallyUsed` (break `SWDiffParams` _output_get))) (`|GetEnumeratorNameAsString` (`.AlgorithmWanted` (break `SWDiffParams` _output_get))) (`.LogRegReady` (break `SWDiffParams` _output_get)) (`.LRAccuracy` (break `SWDiffParams` _output_get)) (`.NbAttemptsUsedToCompute` (break `SWDiffParams` _output_get)))))
    (`|ExecutionSequence`
      (:`then_0`
        (`KismetArrayLibrary.Array_Add` (`self.Thetas`) (`.Theta` (break `SWDiffParams` _output_get))))
      (:`then_1`
        (`KismetArrayLibrary.Array_Add` (`self.Accuracies`) (`.LRAccuracy` (break `SWDiffParams` _output_get))))
      (:`then_2`
        (`KismetArrayLibrary.Array_Add` (`self.Used`) (`.LogRegReady` (break `SWDiffParams` _output_get))))
      (:`then_3`
        (`KismetArrayLibrary.Array_Add` (`self.TargetDiff`) (`.TargetDiffWithExplo` (break `SWDiffParams` _output_get))))
      (:`then_4`
        ;[1 1 1] On fait jouer
        (set `local.Win` (`self.PlayerPlays` (`.Theta` (break `SWDiffParams` _output_get))))
        (`|ExecutionSequence`
          (:`then_0`
            (switch `int` JunkDataType
              (:`1`
                (set `local.Win` (> (`KismetMathLibrary.RandomFloat`) 0.5)))
              (:`2`
                (set `local.Win` true))
              (:`3`
                (set `local.Win` false))))
          (:`then_1`
            (`KismetSystemLibrary.PrintString` (`KismetMathLibrary.SelectString` "win !!" "fail !!" (`local.Win`)))
            (bind _returnvalue (`|GenericCreateObject` "/Script/Swarms.SWDDAAttempt" self))
            (bind _output_get_2 (set `local.Attempt` _returnvalue))
            (set `SWDDAAttempt.Result` (`KismetMathLibrary.SelectFloat` 1.0 0.0 (`local.Win`)) _output_get_2)
            (set `SWDDAAttempt.Thetas` (`|MakeArray` (`.Theta` (break `SWDiffParams` _output_get))) _output_get_2)
            (`/Game/SWARMS/DDA/BP_DDAModelUEBridge.AddLastAttempt` (`self.Dda`) (`local.Attempt`))))))))

(fn `UserConstructionScript`)